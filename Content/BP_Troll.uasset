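; BP_Troll is a troll monster Blueprint that sets its monster name on BeginPlay after calling its parent.
; Three attack events each run a forward multi-sphere trace against pawns, with their own reach, radius and damage, and apply point damage to hits that cast to HT_BaseCharacter.
; The traces leave timed debug drawing enabled, and nothing in this graph triggers the attack events.
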(event Custom|Attack03
  (bind _returnvalue (Transformation|GetActorLocation))
  (bind (_outhits _returnvalue_2) (Collision|MultiSphereTraceForObjects _returnvalue (+ (* (Transformation|GetActorForwardVector) 1.4e+02) _returnvalue) 5e+01 (Utilities|Array|MakeArray "ObjectTypeQuery3") false 0 "ForDuration"))
  (if _returnvalue_2
    (for _array_element _outhits
      (Utilities|Casting|CastToHT_BaseCharacter (.HitActor (Collision|BreakHitResult _array_element)))
      (Game|Damage|ApplyPointDamage (.HitActor (Collision|BreakHitResult _array_element)) 1.5e+02 (Transformation|GetActorLocation) _array_element))))

(event Custom|Attack02
  (bind _returnvalue (Transformation|GetActorLocation))
  (bind (_outhits _returnvalue_2) (Collision|MultiSphereTraceForObjects _returnvalue (+ (* (Transformation|GetActorForwardVector) 9e+01) _returnvalue) 4e+01 (Utilities|Array|MakeArray "ObjectTypeQuery3") false 0 "ForDuration"))
  (if _returnvalue_2
    (for _array_element _outhits
      (Utilities|Casting|CastToHT_BaseCharacter (.HitActor (Collision|BreakHitResult _array_element)))
      (Game|Damage|ApplyPointDamage (.HitActor (Collision|BreakHitResult _array_element)) 8e+01 (Transformation|GetActorLocation) _array_element))))

(event Custom|Attack01
  (bind _returnvalue (Transformation|GetActorLocation))
  (bind (_outhits _returnvalue_2) (Collision|MultiSphereTraceForObjects _returnvalue (+ (* (Transformation|GetActorForwardVector) 125.0) _returnvalue) 5e+01 (Utilities|Array|MakeArray "ObjectTypeQuery3") false 0 "ForDuration"))
  (if _returnvalue_2
    (for _array_element _outhits
      (Utilities|Casting|CastToHT_BaseCharacter (.HitActor (Collision|BreakHitResult _array_element)))
      (Game|Damage|ApplyPointDamage (.HitActor (Collision|BreakHitResult _array_element)) 1e+02 (Transformation|GetActorLocation) _array_element))))

(event EventBeginPlay
  (|CallParentFunction)
  (Variables|Default|SetMonsterName "Troll"))

(fn ConstructionScript)