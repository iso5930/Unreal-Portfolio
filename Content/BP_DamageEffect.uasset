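; BP_DamageEffect is a short-lived floating damage number actor that shows a damage value through a widget component.
; Each Tick re-aligns the actor's X axis along the camera-to-widget direction and drifts it along its up vector.
; A positive damage value is truncated to an integer, passed to BP_DamageWidget, then zeroed so it is not re-sent.
; An accumulated timer destroys the actor after about half a second.
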(event EventBeginPlay)

(event Collision|EventActorBeginOverlap
  (params (OtherActor :type Actor%20Object%20Reference)))

(event EventTick
  (params (DeltaSeconds :type Float%20%28single-precision%29))
  (Transformation|SetActorRotation (Math|Rotator|MakeRotfromX (- (Transformation|GetWorldLocation (Variables|Default|GetDamageWidget)) (Transformation|GetActorLocation (Game|GetPlayerCameraManager 0)))))
  (Transformation|SetActorLocation (+ (Transformation|GetActorLocation) (* (* (Transformation|GetActorUpVector) 5e+01) DeltaSeconds)) false false)
  (bind _output_get (Variables|Default|SetAccTime (+ (Variables|Default|GetAccTime) DeltaSeconds)))
  (if (> _output_get 0.5)
    (Actor|DestroyActor)
    (elif (> (Variables|Default|GetDamege) 0.0)
      (bind _asbp_damage_widget (Utilities|Casting|CastToBP_DamageWidget (UserInterface|GetUserWidgetObject (Variables|Default|GetDamageWidget))))
      (Variables|/Script/Hunter.HT_DamageWidget|SetDamage _asbp_damage_widget (Math|Float|Truncate (Variables|Default|GetDamege)))
      (Variables|Default|SetDamege 0.0))))

(fn ConstructionScript)