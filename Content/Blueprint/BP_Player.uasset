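; Player character Blueprint that handles melee attack hit detection and point damage against HT_BaseMonster enemies.
; Scythe strong attacks sphere-trace forward with damage scaled by player state.
; Other weapons use sphere overlaps with a dot-product facing check, skipped for strong attacks in STATEATTACK01, which hit all around.
; Four attack collision components forward overlaps to a shared weapon handler, and BeginPlay caches the name widget before calling ParentBeginPlay.
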(event OnComponentBeginOverlap(AttackCollision_02)
  (params (OverlappedComponent :type Primitive%20Component%20Object%20Reference) (OtherActor :type Actor%20Object%20Reference) (OtherComp :type Primitive%20Component%20Object%20Reference) (OtherBodyIndex :type Integer) (bFromSweep :type Boolean) (SweepResult :type Hit%20Result%20Structure%20%28by%20ref%29))
  (Class|HTBaseCharacter|OnWeaponAttackOverlap OverlappedComponent OtherActor OtherComp OtherBodyIndex bFromSweep SweepResult))

(event OnComponentBeginOverlap(AttackCollision_03)
  (params (OverlappedComponent :type Primitive%20Component%20Object%20Reference) (OtherActor :type Actor%20Object%20Reference) (OtherComp :type Primitive%20Component%20Object%20Reference) (OtherBodyIndex :type Integer) (bFromSweep :type Boolean) (SweepResult :type Hit%20Result%20Structure%20%28by%20ref%29))
  (Class|HTBaseCharacter|OnWeaponAttackOverlap OverlappedComponent OtherActor OtherComp OtherBodyIndex bFromSweep SweepResult))

(event OnComponentBeginOverlap(AttackCollision_04)
  (params (OverlappedComponent :type Primitive%20Component%20Object%20Reference) (OtherActor :type Actor%20Object%20Reference) (OtherComp :type Primitive%20Component%20Object%20Reference) (OtherBodyIndex :type Integer) (bFromSweep :type Boolean) (SweepResult :type Hit%20Result%20Structure%20%28by%20ref%29))
  (Class|HTBaseCharacter|OnWeaponAttackOverlap OverlappedComponent OtherActor OtherComp OtherBodyIndex bFromSweep SweepResult))

(event OnComponentBeginOverlap(AttackCollision_01)
  (params (OverlappedComponent :type Primitive%20Component%20Object%20Reference) (OtherActor :type Actor%20Object%20Reference) (OtherComp :type Primitive%20Component%20Object%20Reference) (OtherBodyIndex :type Integer) (bFromSweep :type Boolean) (SweepResult :type Hit%20Result%20Structure%20%28by%20ref%29))
  (Class|HTBaseCharacter|OnWeaponAttackOverlap OverlappedComponent OtherActor OtherComp OtherBodyIndex bFromSweep SweepResult))

(event Custom|DualAttackBegin
  (bind _outactors (Collision|SphereOverlapActors (Transformation|GetActorLocation) 8e+01 (Utilities|Array|MakeArray "ObjectTypeQuery3") "/Script/Hunter.HT_BaseMonster"))
  (for _array_element _outactors
    (if (> (Class|Actor|GetDotProductto _array_element) 0.5)
      (Game|Damage|ApplyPointDamage _array_element 5e+01 (Transformation|GetActorForwardVector) (Collision|MakeHitResult false false 0.0 "0, 0, 0" "0, 0, 0" "0,0,1" "0,0,1" 0 0 0) 0 self)
      (Class|HTBaseCharacter|RenderHitEffect))))

(event Custom|StrongAttackBegin
  (bind _returnvalue (Transformation|GetActorLocation))
  (bind _weapon (Variables|Default|GetWeapon))
  (Utilities|IsValid _weapon
    (:Is%20Valid
      (bind _returnvalue_2 (Class|HTBaseWeapon|GetWeaponType _weapon))
      (if (Utilities|Enum|Equal(Enum) _returnvalue_2 "WEAPON_SCYTHE")
        (bind _outhits (Collision|MultiSphereTraceForObjects _returnvalue (+ (* (Transformation|GetActorForwardVector) 7e+01) _returnvalue) 5e+01 (Utilities|Array|MakeArray "ObjectTypeQuery3") false 0 "ForDuration"))
        (for _array_element _outhits
          (Utilities|Casting|CastToHT_BaseMonster (.HitActor (Collision|BreakHitResult _array_element)))
          (bind _returnvalue_3 (Class|HTBaseCharacter|GetCurPlayerState))
          (Game|Damage|ApplyPointDamage (.HitActor (Collision|BreakHitResult _array_element)) (+ (* 2e+01 (Math|Conversions|ToFloat(Byte) _returnvalue_3)) 1e+01) (Transformation|GetActorForwardVector) _array_element 0 self)
          (Class|HTBaseCharacter|RenderHitEffect))
        (else
          (bind _outactors (Collision|SphereOverlapActors (Transformation|GetActorLocation) 8e+01 (Utilities|Array|MakeArray "ObjectTypeQuery3") "/Script/Hunter.HT_BaseMonster"))
          (for _array_element_2 _outactors
            (bind _returnvalue_4 (Class|HTBaseCharacter|GetCurPlayerState))
            (if (Utilities|Enum|Equal(Enum) _returnvalue_4 "PLAYER_STATE_ATTACK01")
              (|DualBladeStrongAttack01 _array_element_2)
              (elif (> (Class|Actor|GetDotProductto _array_element_2) 0.5)
                (Game|Damage|ApplyPointDamage _array_element_2 5e+01 (Transformation|GetActorForwardVector) (Collision|MakeHitResult false false 0.0 "0, 0, 0" "0, 0, 0" "0,0,1" "0,0,1" 0 0 0) 0 self)
                (Class|HTBaseCharacter|RenderHitEffect)))))))))

(event Game|Damage|EventPointDamage
  (params (Damage :type Float%20%28single-precision%29) (DamageType :type Damage%20Type%20Object%20Reference) (HitLocation :type Vector :default "0, 0, 0") (HitNormal :type Vector :default "0, 0, 0") (HitComponent :type Primitive%20Component%20Object%20Reference) (BoneName :type Name :default "None") (ShotFromDirection :type Vector :default "0, 0, 0") (InstigatedBy :type Controller%20Object%20Reference) (DamageCauser :type Actor%20Object%20Reference) (HitInfo :type Hit%20Result%20Structure%20%28by%20ref%29))
  (Class|HTBaseCharacter|PointDamage Damage))

(event EventBeginPlay
  (bind _asht_user_name_widget (Utilities|Casting|CastToHT_UserNameWidget (UserInterface|GetUserWidgetObject (Variables|Default|GetNameWidget)))
    (:then
      (Variables|Default|SetUserNameWidget _asht_user_name_widget)
      (|CallParentFunction))
    (:CastFailed
      (|CallParentFunction))))

(fn ConstructionScript)