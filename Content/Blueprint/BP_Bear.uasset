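; BP_Bear is a monster Blueprint that names itself "Bear" on BeginPlay after running the parent's setup.
; Its AttackBegin event runs a short multi-sphere trace for Pawns forward from the bear's location.
; Each hit that casts to HT_BaseCharacter takes fixed point damage, and the first failed cast is written to stop that path.
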(event Custom|AttackBegin
  (bind _returnvalue (Transformation|GetActorLocation))
  (bind (_outhits _returnvalue_2) (Collision|MultiSphereTraceForObjects _returnvalue (+ (* (Transformation|GetActorForwardVector) 8e+01) _returnvalue) 3e+01 (Utilities|Array|MakeArray "ObjectTypeQuery3") false 0 "None"))
  (if _returnvalue_2
    (for _array_element _outhits
      (Utilities|Casting|CastToHT_BaseCharacter (.HitActor (Collision|BreakHitResult _array_element)))
      (Game|Damage|ApplyPointDamage (.HitActor (Collision|BreakHitResult _array_element)) 6e+01 (Transformation|GetActorLocation) _array_element))))

(event EventBeginPlay
  (|CallParentFunction)
  (Variables|Default|SetMonsterName "Bear"))

(fn ConstructionScript)