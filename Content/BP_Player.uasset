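; BP_Player is the player character Blueprint, a thin layer over a parent class that handles name display and weapon hit detection.
; On BeginPlay it caches the NameWidget component's HT_UserNameWidget before calling the parent's BeginPlay.
; Four attack collision components forward their begin-overlap events to a shared OnWeaponAttackOverlap handler.
; PointDamage events pass their damage straight on to a PointDamage call.
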(event OnComponentBeginOverlap(AttackCollision_02)
  (params (OverlappedComponent :type Primitive%20Component%20Object%20Reference) (OtherActor :type Actor%20Object%20Reference) (OtherComp :type Primitive%20Component%20Object%20Reference) (OtherBodyIndex :type Integer) (bFromSweep :type Boolean) (SweepResult :type Hit%20Result%20Structure%20%28by%20ref%29))
  (Class|HTBaseCharacter|OnWeaponAttackOverlap OverlappedComponent OtherActor OtherComp OtherBodyIndex bFromSweep SweepResult))

(event OnComponentBeginOverlap(AttackCollision_03)
  (params (OverlappedComponent :type Primitive%20Component%20Object%20Reference) (OtherActor :type Actor%20Object%20Reference) (OtherComp :type Primitive%20Component%20Object%20Reference) (OtherBodyIndex :type Integer) (bFromSweep :type Boolean) (SweepResult :type Hit%20Result%20Structure%20%28by%20ref%29))
  (Class|HTBaseCharacter|OnWeaponAttackOverlap OverlappedComponent OtherActor OtherComp OtherBodyIndex bFromSweep SweepResult))

(event OnComponentBeginOverlap(AttackCollision_04)
  (params (OverlappedComponent :type Primitive%20Component%20Object%20Reference) (OtherActor :type Actor%20Object%20Reference) (OtherComp :type Primitive%20Component%20Object%20Reference) (OtherBodyIndex :type Integer) (bFromSweep :type Boolean) (SweepResult :type Hit%20Result%20Structure%20%28by%20ref%29))
  (Class|HTBaseCharacter|OnWeaponAttackOverlap OverlappedComponent OtherActor OtherComp OtherBodyIndex bFromSweep SweepResult))

(event OnComponentBeginOverlap(AttackCollision_01)
  (params (OverlappedComponent :type Primitive%20Component%20Object%20Reference) (OtherActor :type Actor%20Object%20Reference) (OtherComp :type Primitive%20Component%20Object%20Reference) (OtherBodyIndex :type Integer) (bFromSweep :type Boolean) (SweepResult :type Hit%20Result%20Structure%20%28by%20ref%29))
  (Class|HTBaseCharacter|OnWeaponAttackOverlap OverlappedComponent OtherActor OtherComp OtherBodyIndex bFromSweep SweepResult))

(event Game|Damage|EventPointDamage
  (params (Damage :type Float%20%28single-precision%29) (DamageType :type Damage%20Type%20Object%20Reference) (HitLocation :type Vector :default "0, 0, 0") (HitNormal :type Vector :default "0, 0, 0") (HitComponent :type Primitive%20Component%20Object%20Reference) (BoneName :type Name :default "None") (ShotFromDirection :type Vector :default "0, 0, 0") (InstigatedBy :type Controller%20Object%20Reference) (DamageCauser :type Actor%20Object%20Reference) (HitInfo :type Hit%20Result%20Structure%20%28by%20ref%29))
  (Class|HTBaseCharacter|PointDamage Damage))

(event EventBeginPlay
  (bind _asht_user_name_widget (Utilities|Casting|CastToHT_UserNameWidget (UserInterface|GetUserWidgetObject (Variables|Default|GetNameWidget)))
    (:then
      (Variables|Default|SetUserNameWidget _asht_user_name_widget)
      (|CallParentFunction))
    (:CastFailed
      (|CallParentFunction))))

(fn ConstructionScript)